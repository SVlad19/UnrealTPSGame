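; BP_TPSInventoryItem is an inventory item actor whose look is built from its InventoryData.
; The construction script calls Init, which picks a primitive mesh from the item Type and shows the Score on a text render.
; GenerateColor draws a random ColorPalette entry, applied to both a dynamic material instance and the text.
; On EndPlay it spawns a Niagara explosion at the actor's location, whatever the end reason.
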(event `self.ReceiveEndPlay`
  (params (EndPlayReason :type "EEndPlayReason Enum" :default "Destroyed"))
  (`NiagaraFunctionLibrary.SpawnSystemAtLocation` "/Game/Inventory/NS_Explosion.NS_Explosion" (`self.K2_GetActorLocation`)))

(fn `GenerateColor`
  (returns (Color :type "LinearColor Structure"))
  (return (`KismetArrayLibrary.Array_Random` (`self.Color Palette`))))

(fn `Init`
  (locals (ColorToSet :type "LinearColor Structure"))
  (bind (_inventorydata_type _inventorydata_score) (break `InventoryData` (`self.InventoryData`)))
  (`StaticMeshComponent.SetStaticMesh` (`self.StaticMesh`) (select `EInventoryItemType` _inventorydata_type :`SPHERE` "/Engine/BasicShapes/Sphere.Sphere" :`CUBE` "/Engine/BasicShapes/Cube.Cube" :`CYLINDER` "/Engine/BasicShapes/Cylinder.Cylinder" :`CONE` "/Engine/BasicShapes/Cone.Cone" :!type "StaticMesh Object Reference"))
  (`TextRenderComponent.K2_SetText` (`self.TextRender`) (`KismetTextLibrary.Conv_IntToText` _inventorydata_score))
  (bind _returnvalue (`PrimitiveComponent.CreateDynamicMaterialInstance` (`self.StaticMesh`) 0 "/Game/Materials/M_BaseColor.M_BaseColor" "None"))
  (bind _output_get (set `local.ColorToSet` (`self.GenerateColor`)))
  (`MaterialInstanceDynamic.SetVectorParameterValue` _returnvalue "Color" _output_get)
  (`TextRenderComponent.SetTextRenderColor` (`self.TextRender`) (`KismetMathLibrary.Conv_LinearColorToColor` (`local.ColorToSet`))))

(fn `UserConstructionScript`
  (`self.Init`))